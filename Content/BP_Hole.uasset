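; BP_Hole is an actor that shows a hole mesh and probes the surface beneath it.
; Its construction script assigns the mesh, prints the spawn location and adds itself to the trace ignore list.
; On BeginPlay it runs a short downward Visibility line trace with debug drawing and prints the hit actor's name.
; A check for a Landscape hit follows, but its branch is empty.
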(event `self.ReceiveBeginPlay`
  (bind _returnvalue (`self.K2_GetActorLocation`))
  (bind _outhit (`KismetSystemLibrary.LineTraceSingle` (+ _returnvalue (0.0 0.0 5.0)) (- _returnvalue (0.0 0.0 100.0)) "TraceTypeQuery1" false (`self.Actors to Ignore`) "ForDuration"))
  (bind (_bblockinghit _binitialoverlap _time _distance _location _impactpoint _normal _impactnormal _physmat _hitactor) (`GameplayStatics.BreakHitResult` _outhit))
  (`KismetSystemLibrary.PrintString` (`KismetSystemLibrary.GetDisplayName` _hitactor))
  (if (`GameplayStatics.ObjectIsA` _hitactor "/Script/Landscape.LandscapeProxy")
    _))

(fn `UserConstructionScript`
  (`StaticMeshComponent.SetStaticMesh` (`self.StaticMeshComponent`) (`self.HoleMesh`))
  (`KismetSystemLibrary.PrintString` (`KismetStringLibrary.BuildString_Vector` "Hole spawned at location:" "" (`self.K2_GetActorLocation`)))
  (set `self.Actors to Ignore` (`|MakeArray` self :!type "Actor Object Reference")))