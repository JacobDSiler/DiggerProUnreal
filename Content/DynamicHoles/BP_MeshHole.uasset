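; BP_MeshHole is an actor for a dynamic mesh hole that lets overlapping pawns pass through the landscape.
; InitializeHoleMesh assigns a supplied mesh to both the StaticMesh and Overlay components, each with its own material.
; Begin and end overlap send messages to the other actor to enable landscape pass-through, then restore default collision.
; BeginPlay runs a visibility line trace from its location and prints the hit actor for debugging.
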(event `self.ReceiveBeginPlay`
  (bind _outhit (`KismetSystemLibrary.LineTraceSingle` (`self.K2_GetActorLocation`) (0.0 0.0 0.0) "TraceTypeQuery1"))
  (`KismetSystemLibrary.PrintString` (`KismetStringLibrary.Concat_StrStr` "Hit actor: " (`KismetSystemLibrary.GetDisplayName` (`.HitActor` (`GameplayStatics.BreakHitResult` _outhit))))))

(event `self.ReceiveActorBeginOverlap`
  (params (OtherActor :type "Actor Object Reference"))
  (message `/Game/DynamicHoles/BPI_PassPawnThroughLandscape.SetPawnPassThroughLandscape` OtherActor))

(event `self.ReceiveActorEndOverlap`
  (params (OtherActor :type "Actor Object Reference"))
  (message `/Game/DynamicHoles/BPI_PassPawnThroughLandscape.ResetPawnDefaultCollision` OtherActor))

(fn `InitializeHoleMesh`
  (params (HoleMesh :type "StaticMesh Object Reference"))
  ;[1 1 1] Dynamic Mesh for the hole.
  (`StaticMeshComponent.SetStaticMesh` (`self.StaticMesh`) HoleMesh)
  (`PrimitiveComponent.SetMaterial` (`self.StaticMesh`) 0 (`self.Material`))
  ;[1 1 1] Overlay Mesh
  (`StaticMeshComponent.SetStaticMesh` (`self.Overlay`) HoleMesh)
  (`PrimitiveComponent.SetMaterial` (`self.Overlay`) 0 "/Game/Materials/M_Overlay.M_Overlay"))

(fn `UserConstructionScript`)