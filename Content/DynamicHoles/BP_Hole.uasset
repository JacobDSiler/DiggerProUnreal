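; BP_Hole is a placeable hole actor that cuts itself into the landscape beneath it when play begins.
; Its construction script applies the configured hole mesh, and BeginPlay traces a short distance straight down, ignoring itself.
; If the trace hits a landscape, it passes that landscape and its mesh component to MyDiggerManager's DigHole.
; Otherwise it logs a failure and destroys itself.
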(event `self.ReceiveBeginPlay`
  (bind _returnvalue (`self.K2_GetActorLocation`))
  (bind _outhit (`KismetSystemLibrary.LineTraceSingle` (+ _returnvalue (0.0 0.0 5.0)) (- _returnvalue (0.0 0.0 100.0)) "TraceTypeQuery1" false (`self.Actors to Ignore`) "ForDuration"))
  (bind (_bblockinghit _binitialoverlap _time _distance _location _impactpoint _normal _impactnormal _physmat _hitactor) (`GameplayStatics.BreakHitResult` _outhit))
  (`KismetSystemLibrary.PrintString` (`KismetSystemLibrary.GetDisplayName` _hitactor))
  (if (`GameplayStatics.ObjectIsA` _hitactor "/Script/Landscape.LandscapeProxy")
    (bind _aslandscape_proxy (cast `LandscapeProxy` _hitactor))
    (bind _returnvalue_2 (`GameplayStatics.GetActorOfClass` "/Game/BluePrints/MyDiggerManager.MyDiggerManager_C"))
    (`DiggerManager.DigHole` _returnvalue_2 _aslandscape_proxy (`self.StaticMeshComponent`))
    (else
      (`KismetSystemLibrary.PrintString` "No landscape was found by the new hole. :'( Sad day!!!")
      (`self.K2_DestroyActor`))))

(fn `UserConstructionScript`
  (`StaticMeshComponent.SetStaticMesh` (`self.StaticMeshComponent`) (`self.HoleMesh`))
  (`KismetSystemLibrary.PrintString` (`KismetStringLibrary.BuildString_Vector` "Hole spawned at location:" "" (`self.K2_GetActorLocation`)))
  (set `self.Actors to Ignore` (`|MakeArray` self :!type "Actor Object Reference")))