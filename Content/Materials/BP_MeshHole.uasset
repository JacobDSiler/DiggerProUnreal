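; BP_MeshHole is an actor that displays a configurable hole mesh with an overlay.
; Its construction script assigns the HoleMesh variable to both the StaticMesh and Overlay components, so they share one shape.
; StaticMesh takes the Material variable and Overlay takes M_Overlay, each on the first material slot.
; The event graph holds only disabled placeholder events, so the Blueprint adds no runtime logic.
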(fn `UserConstructionScript`
  ;[1 1 1] Dynamic Mesh for the hole.
  (`StaticMeshComponent.SetStaticMesh` (`self.StaticMesh`) (`self.HoleMesh`))
  (`PrimitiveComponent.SetMaterial` (`self.StaticMesh`) 0 (`self.Material`))
  ;[1 1 1] Overlay Mesh
  (`StaticMeshComponent.SetStaticMesh` (`self.Overlay`) (`self.HoleMesh`))
  (`PrimitiveComponent.SetMaterial` (`self.Overlay`) 0 "/Game/Materials/M_Overlay.M_Overlay"))